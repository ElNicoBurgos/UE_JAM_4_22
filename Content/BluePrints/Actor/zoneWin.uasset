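; Win-zone actor that ends the game when the player enters it with enough collected scrap.
; On overlap by MyCharacter, it compares CollectedScraps to the count of MetalScrap actors currently in the level.
; On success it fades the camera out, disables input, shows the WonScreen widget and the mouse cursor.
; A DoOnce with no reset precedes the check, so only the first character overlap is evaluated.
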(event EventBeginPlay)

(event EventTick
  (params (DeltaSeconds :type Float%20%28single-precision%29)))

(event Collision|EventActorBeginOverlap
  (params (OtherActor :type Actor%20Object%20Reference))
  (bind _outactors (Actor|GetAllActorsOfClass "/Game/BluePrints/Actor/Loot/MetalScrap.MetalScrap_C"))
  (bind _asmy_character (Utilities|Casting|CastToMyCharacter OtherActor))
  (Utilities|FlowControl|DoOnce false
    (:Completed
      (bind _asgame_mode_jam (Utilities|Casting|CastToGameModeJam (Game|GetGameMode)))
      (Development|PrintString "Win actor")
      (if (>= (Variables|/Game/BluePrints/Character/MyCharacter.MyCharacter_C|GetCollected%20Scraps _asmy_character) (Utilities|Array|Length _outactors))
        (CameraFades|StartCameraFade :self (Game|GetPlayerCameraManager 0) :ToAlpha 1.0 :Duration 0.3 :bShouldFadeAudio true :bHoldWhenFinished true)
        (Input|DisableInput (Game|Player|GetPlayerPawn 0) (Game|GetPlayerController 0))
        (bind _returnvalue (UserInterface|CreateWidget "/Game/UI/WonScreen.WonScreen_C"))
        (UserInterface|Viewport|AddtoViewport _returnvalue 0)
        (Variables|/Script/Engine.PlayerController|SetbShowMouseCursor (Game|GetPlayerController 0) true)))))

(fn ConstructionScript)