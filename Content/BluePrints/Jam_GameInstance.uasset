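; Game instance Blueprint for a jam game that shows on-screen information messages.
; ShowInformation creates an Info widget from the given duration, text and color, adds it to the viewport, and records that duration and a shown flag.
; The check on that flag has no effect, as both branches lead to immediate display.
; An unconnected delay chain for holding back a second message and resetting the flags never runs.
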(event Custom|Show%20Information
  (params (Duration :type Float%20%28single-precision%29) (Text :type Text) (Color :type Slate%20Color%20Structure))
  (if (Variables|Default|GetHave%20Showed%20Info%20Before?)
    _
    (else
      _))
  (Variables|Default|SetHave%20Showed%20Info%20Before? true)
  (bind _output_get (Variables|Default|SetFirst%20Info%20Duration Duration))
  (bind _returnvalue (UserInterface|CreateWidget "/Game/UI/Info.Info_C" 0 Duration Text Color))
  (UserInterface|Viewport|AddtoViewport _returnvalue 0))