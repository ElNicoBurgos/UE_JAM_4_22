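; 3D settings menu actor that hosts a SettingsWidget in the world through a widget component.
; On BeginPlay it passes itself to that widget as its owning 3D actor reference.
; Its destroy event plays the widget's Show animation in reverse, waits briefly, then removes the actor.
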(event Custom|Destroy%203D%20Settings%20Menu
  (bind _widget (Variables|Default|GetWidget))
  (bind _returnvalue (UserInterface|GetUserWidgetObject _widget))
  (bind _assettings_widget (Utilities|Casting|CastToSettingsWidget _returnvalue))
  (UserInterface|Animation|PlayAnimation _returnvalue (Variables|/Game/UI/SettingsWidget.SettingsWidget_C|GetShow _assettings_widget) 0.0 1 "Reverse" 1.0)
  (Utilities|FlowControl|Delay 0.25)
  (Actor|DestroyActor))

(event EventBeginPlay
  (bind _assettings_widget (Utilities|Casting|CastToSettingsWidget (UserInterface|GetUserWidgetObject (Variables|Default|GetWidget))))
  (Variables|/Game/UI/SettingsWidget.SettingsWidget_C|Set3D%20Widget%20Actor _assettings_widget self))

(fn ConstructionScript)