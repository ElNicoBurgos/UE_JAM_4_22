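; Game jam GameMode that resets the level's Robot and sets the scrap-based win target at BeginPlay.
; It destroys every placed Robot, then spawns one at the last valid RobotSpawnLocation found and has its AI controller possess it.
; After that spawn, the count of MetalScrap actors becomes AmountObjectToWin.
; Player spawn, HUD creation and "einar_1" camera-fade logic are present but disconnected, and PostLogin is empty.
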(event EventTick
  (params (DeltaSeconds :type Float%20%28single-precision%29)))

(event EventPostLogin
  (params (NewPlayer :type Player%20Controller%20Object%20Reference)))

(event EventBeginPlay
  (Utilities|FlowControl|Sequence
    (:then_0
      (bind _outactors (Actor|GetAllActorsOfClass "/Game/BluePrints/Character/Robot.Robot_C"))
      (for _array_element _outactors
        (Actor|DestroyActor _array_element)))
    (:then_1
      (bind _outactors_2 (Actor|GetAllActorsOfClass "/Game/BluePrints/RobotSpawnLocation.RobotSpawnLocation_C"))
      (for _array_element_2 _outactors_2
        _)
      (if (Utilities|IsValid _array_element_2)
        (bind _returnvalue (Game|SpawnActorfromClass "/Game/BluePrints/Character/Robot.Robot_C" (Transformation|GetActorTransform _array_element_2) "AdjustIfPossibleButAlwaysSpawn" 0 0))
        (Pawn|Possess (AI|GetAIController _returnvalue) _returnvalue)
        (bind _outactors_3 (Actor|GetAllActorsOfClass "/Game/BluePrints/Actor/Loot/MetalScrap.MetalScrap_C"))
        (Variables|Default|SetamountObjectToWin (Utilities|Array|Length _outactors_3))))))

(fn ConstructionScript)