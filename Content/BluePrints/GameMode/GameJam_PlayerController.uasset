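; Player controller for a game jam project that owns the HUD and drives a screen color flash.
; It creates the HUD widget on BeginPlay, and DestroyHUD tears it down after a short delay with a debug print of its validity.
; ColorOverlay chains two camera fades to ramp a given color in and back out using damage overlay settings, with the H key triggering a black one.
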(event Custom|Color%20Overlay
  (params (Color :type Linear%20Color%20Structure))
  (bind _returnvalue (Game|GetPlayerCameraManager 0))
  (bind _damage_overlay_power (Variables|Default|GetDamage%20Overlay%20Power))
  (bind _damage_overlay_fade_duration (Variables|Default|GetDamage%20Overlay%20Fade%20Duration))
  (CameraFades|StartCameraFade _returnvalue 0.0 _damage_overlay_power _damage_overlay_fade_duration Color false false)
  (Utilities|FlowControl|Delay _damage_overlay_fade_duration)
  (CameraFades|StartCameraFade _returnvalue _damage_overlay_power 0.0 _damage_overlay_fade_duration Color false false))

(event Custom|Destroy%20HUD
  (bind _hud_reference (Variables|Default|GetHUD%20Reference))
  (Utilities|FlowControl|Delay 0.2)
  (Default|DestroyHUDInternal _hud_reference)
  (Development|PrintString (Utilities|String|ToString(Boolean) (Utilities|IsValid _hud_reference)) true true "(R=0.104774,G=1.000000,B=0.000000,A=1.000000)"))

(event Custom|Create%20HUD
  (bind _returnvalue (UserInterface|CreateWidget "/Game/UI/HUD.HUD_C" self))
  (bind _output_get (Variables|Default|SetHUD%20Reference _returnvalue))
  (UserInterface|Viewport|AddtoViewport _output_get 0))

(event EventBeginPlay
  (CallFunction|CreateHUD))

(event Input|KeyboardEvents|H
  (params (Key :type Key%20Structure))
  (:Pressed
    (CallFunction|ColorOverlay)))

(fn ConstructionScript)