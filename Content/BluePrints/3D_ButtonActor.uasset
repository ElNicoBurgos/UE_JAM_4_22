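; 3D_ButtonActor is a world-space menu button whose ButtonType selects a Play, Settings or Quit label.
; On BeginPlay it caches the 3DButtonWidget from its ButtonWidget component and passes itself to it as a back-reference.
; Tick reapplies label and half scale every frame, and the construction script sets the label if the cached widget is valid.
; DestroyButton plays the widget's Show animation in reverse, then destroys the actor after a short delay.
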(event Custom|Destroy%20Button
  (bind _button_widget (Variables|Default|GetButton%20Widget))
  (bind _returnvalue (UserInterface|GetUserWidgetObject _button_widget))
  (bind _as3dbutton_widget (Utilities|Casting|CastTo3DButtonWidget _returnvalue))
  (UserInterface|Animation|PlayAnimation _returnvalue (Variables|/Game/UI/3DButtonWidget.3DButtonWidget_C|GetShow _as3dbutton_widget) 0.0 1 "Reverse" 1.0)
  (Utilities|FlowControl|Delay 0.2)
  (Actor|DestroyActor))

(event EventBeginPlay
  (bind _as3dbutton_widget (Utilities|Casting|CastTo3DButtonWidget (UserInterface|GetUserWidgetObject (Variables|Default|GetButton%20Widget))))
  (Variables|/Game/UI/3DButtonWidget.3DButtonWidget_C|Set3D%20Button%20Actor _as3dbutton_widget self)
  (Variables|Default|Set3D%20Button%20Widget _as3dbutton_widget))

(event EventTick
  (params (DeltaSeconds :type Float%20%28single-precision%29))
  (bind _button_type (Variables|Default|GetButton%20Type))
  (bind _returnvalue (Utilities|Select :Index _button_type :NewEnumerator0 0.5 :NewEnumerator1 0.5 :NewEnumerator2 0.5))
  (Default|Set3DButtonText (Variables|Default|Get3D%20Button%20Widget) (Utilities|Select :Index _button_type :NewEnumerator0 "Play" :NewEnumerator1 "Settings" :NewEnumerator2 "Quit"))
  (Transformation|SetActorScale3D (Math|Vector|MakeVector _returnvalue _returnvalue _returnvalue)))

(fn ConstructionScript
  (bind _3d_button_widget (Variables|Default|Get3D%20Button%20Widget))
  (Utilities|IsValid _3d_button_widget
    (:Is%20Valid
      (Default|Set3DButtonText _3d_button_widget (Utilities|Select :Index (Variables|Default|GetButton%20Type) :NewEnumerator0 "Play" :NewEnumerator1 "Settings" :NewEnumerator2 "Quit")))))