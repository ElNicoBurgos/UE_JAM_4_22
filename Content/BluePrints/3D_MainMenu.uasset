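; 3D main menu actor that presents the MainMenu user widget through a widget component.
; On BeginPlay it passes a reference to itself into that MainMenu widget.
; Its Destroy3DMainMenu event plays the widget's Spawn animation in reverse, waits briefly, then destroys the actor.
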(event Custom|Destroy%203D%20Main%20Menu
  (bind _widget (Variables|Default|GetWidget))
  (bind _returnvalue (UserInterface|GetUserWidgetObject _widget))
  (bind _asmain_menu (Utilities|Casting|CastToMainMenu _returnvalue))
  (UserInterface|Animation|PlayAnimation _returnvalue (Variables|/Game/UI/MainMenu.MainMenu_C|GetSpawn _asmain_menu) 0.0 1 "Reverse" 1.0)
  (Utilities|FlowControl|Delay 0.5)
  (Actor|DestroyActor))

(event EventBeginPlay
  (bind _asmain_menu (Utilities|Casting|CastToMainMenu (UserInterface|GetUserWidgetObject (Variables|Default|GetWidget))))
  (Variables|/Game/UI/MainMenu.MainMenu_C|Set3D%20Main%20Menu%20Actor _asmain_menu self))

(fn ConstructionScript)