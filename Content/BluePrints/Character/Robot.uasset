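; Companion robot character that follows the player, travels to commanded locations and plays loot and pickup effects.
; Each Tick it either snaps to the player's AILocation, banking its spring arm with movement input or facing the idle player, or detaches for an AI MoveToLocation.
; An accepted or already-completed move request immediately calls ResetRobotMission on the player.
; PickUpObject uses a timeline to pull the item into the mesh, shrink and destroy it.
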(event Custom|Disable%20Loot%20Effects
  (Components|Activation|SetActive (Variables|Default|GetStyleLight1) false false))

(event Custom|Enable%20Loot%20Effects
  (Components|Activation|SetActive (Variables|Default|GetStyleLight2) true false))

(event Custom|Pick%20Up%20Object
  (bind _object_to_pick_up (Variables|Default|GetObject%20To%20Pick%20Up))
  (bind _lerp (Timeline|Pick%20Up%20Effects PlayFromStart)
    (:Update
      (Utilities|FlowControl|Sequence
        (:then_0
          (Utilities|FlowControl|DoOnce false :!label _label
            (:Completed
              (Variables|Default|SetPicked%20up%20object's%20location%20before%20effects (Transformation|GetActorLocation _object_to_pick_up)))))
        (:then_1
          (Transformation|SetActorLocation _object_to_pick_up (Math|Vector|Lerp(Vector) (Variables|Default|GetPicked%20up%20object's%20location%20before%20effects) (Transformation|GetWorldLocation (Variables|Default|GetSkeletalMesh)) _lerp) false false)
          (Transformation|SetActorScale3D _object_to_pick_up (Math|Vector|Lerp(Vector) "1.000000,1.000000,1.000000" "0.250000,0.250000,0.250000" _lerp)))))
    (:Finished
      (Actor|DestroyActor _object_to_pick_up)
      (goto _label Reset))))

(event EventTick
  (params (DeltaSeconds :type Float%20%28single-precision%29))
  (bind _returnvalue (Game|Player|GetPlayerPawn 0))
  (bind _returnvalue_2 (Game|GetPlayerCharacter 0))
  (bind _self self)
  (bind _returnvalue_3 (Transformation|GetVelocity _returnvalue))
  (bind _returnvalue_4 (AI|GetAIController _self))
  (bind _asmy_character (Utilities|Casting|CastToMyCharacter _returnvalue_2))
  (bind (_x _y) (Math|Vector|BreakVector _returnvalue_3))
  (bind _right_axis (Variables|/Game/BluePrints/Character/MyCharacter.MyCharacter_C|GetRight%20Axis _asmy_character))
  (bind _returnvalue_5 (> _right_axis 0.1))
  (bind _returnvalue_6 (< _right_axis -0.1))
  (Utilities|FlowControl|Sequence
    (:then_0
      (if (Variables|Default|GetIs%20There%20a%20Command)
        (Transformation|DetachFromActor "KeepWorld" "KeepRelative" "KeepRelative")
        (else
          (bind _asmy_character_2 (Utilities|Casting|CastToMyCharacter (Game|GetPlayerCharacter 0)))
          (Transformation|AttachComponentToComponent (Variables|/Game/BluePrints/Character/MyCharacter.MyCharacter_C|GetAI%20location _asmy_character_2) "None" "SnapToTarget" "SnapToTarget" "KeepRelative" true))))
    (:then_1
      (if (Variables|Default|GetIs%20There%20a%20Command)
        (bind _returnvalue_7 (AI|Navigation|MovetoLocation (AI|GetAIController self) (Variables|Default|GetCommand%20Location) -1.0 true true true true 0))
        (switch Utilities|FlowControl|Switch|SwitchonEPathFollowingRequestResult _returnvalue_7
          (:Failed
            (Variables|Default|SetIs%20There%20a%20Command false))
          (:AlreadyAtGoal
            (bind _asmy_character_3 (Utilities|Casting|CastToMyCharacter (Game|GetPlayerCharacter 0) :!label _label))
            (Default|ResetRobotMission _asmy_character_3))
          (:RequestSuccessful
            (goto _label)))
        (elif (> (Math|Vector|VectorLength (Math|Vector|MakeVector _x _y 0.0)) 0.0)
          (Pawn|SetControlRotation _returnvalue_4 (Pawn|GetControlRotation (Game|GetPlayerController 0) :!class /Script/Engine.Controller))
          (bind _output_get (Variables|Default|SetSmoothed%20Rotation (Math|Interpolation|RInterpTo (stale _output_get) (select (> (Variables|/Game/BluePrints/Character/MyCharacter.MyCharacter_C|GetForward%20Axis _asmy_character) 0.0) (select _returnvalue_5 "0,35.000000,0.000000" (select _returnvalue_6 "0,-35.000000,0.000000" "0, 0, 0")) (select _returnvalue_5 "0.000000,60.000000,0.000000" (select _returnvalue_6 "0,-60.000000,0.000000" "0, 0, 0"))) (Utilities|Time|GetWorldDeltaSeconds) 15.0)))
          (Transformation|SetRelativeRotation (Variables|Default|GetSpringArm) _output_get false false)
          (else
            (Pawn|SetControlRotation _returnvalue_4 (Math|Rotator|FindLookatRotation (Transformation|GetActorLocation) (Transformation|GetActorLocation (Game|GetPlayerCharacter 0))))))))
    (:then_2
      (Development|PrintString (Utilities|String|ToString(Boolean) (Variables|Default|GetIs%20There%20a%20Command))))))

(fn ConstructionScript)