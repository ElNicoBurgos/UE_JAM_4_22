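; MovingStar is an actor whose Star component is driven along negative Y, faster as a tracked marker actor gets nearer.
; On BeginPlay it takes the first EmptyActor found as the player location reference.
; Each tick it maps the clamped distance to that actor into an alpha, blends from very high to much lower velocity, overwrites the physics linear velocity and prints the alpha.
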(event EventTick
  (params (DeltaSeconds :type Float%20%28single-precision%29))
  (bind _actor_that_determines_player_location (Variables|Default|GetActor%20That%20determines%20player%20location))
  (bind _returnvalue (Transformation|GetDistanceTo _actor_that_determines_player_location))
  (bind _returnvalue_2 (Math|Float|MapRangeClamped _returnvalue 5e+01 1e+03 0.0 1.0))
  (bind _returnvalue_3 (Math|Float|Lerp 0.0 1.0 _returnvalue_2))
  (Physics|SetPhysicsLinearVelocity (Variables|Default|GetStar) (Math|Vector|Lerp(Vector) "0,-100000.000000, 0" "0,-1000.000000, 0" _returnvalue_3) false "None")
  (Development|PrintString (Utilities|String|ToString(Float) _returnvalue_3) true true "(R=0.000000,G=0.660000,B=1.000000,A=1.000000)" 0.0))

(event EventBeginPlay
  (bind _outactors (Actor|GetAllActorsOfClass "/Game/BluePrints/EmptyActor.EmptyActor_C"))
  (Variables|Default|SetActor%20That%20determines%20player%20location (Utilities|Array|Get(acopy) _outactors)))

(fn ConstructionScript)