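; 3D menu button actor that shows Play, Settings or Quit text through a 3DButton user widget, based on its ButtonType.
; On BeginPlay it passes itself to the widget and caches it for later calls.
; The label is set in the construction script and re-applied every Tick, along with a uniform actor scale.
; DestroyButton reverses the widget's Show animation, then destroys the actor after a short delay.
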(event Custom|Destroy%20Button
  (bind _widget (Variables|Default|GetWidget))
  (bind _returnvalue (UserInterface|GetUserWidgetObject _widget))
  (bind _as3dbutton (Utilities|Casting|CastTo3DButton _returnvalue))
  (UserInterface|Animation|PlayAnimation _returnvalue (Variables|/Game/UI/3DButton.3DButton_C|GetShow _as3dbutton) 0.0 1 "Reverse" 1.0)
  (Utilities|FlowControl|Delay 0.2)
  (Actor|DestroyActor))

(event EventBeginPlay
  (bind _as3dbutton (Utilities|Casting|CastTo3DButton (UserInterface|GetUserWidgetObject (Variables|Default|GetWidget))))
  (Variables|/Game/UI/3DButton.3DButton_C|Set3D%20Button%20Actor _as3dbutton self)
  (Variables|Default|Set3D%20Button%20Widget _as3dbutton))

(event EventTick
  (params (DeltaSeconds :type Float%20%28single-precision%29))
  (bind _button_type (Variables|Default|GetButton%20Type))
  (bind _returnvalue (Utilities|Select :Index _button_type :NewEnumerator0 0.5 :NewEnumerator1 0.5 :NewEnumerator2 0.5))
  (Default|Set3DButtonText (Variables|Default|Get3D%20Button%20Widget) (Utilities|Select :Index _button_type :NewEnumerator0 "Play" :NewEnumerator1 "Settings" :NewEnumerator2 "Quit"))
  (Transformation|SetActorScale3D (Math|Vector|MakeVector _returnvalue _returnvalue _returnvalue)))

(fn ConstructionScript
  (Default|Set3DButtonText (Variables|Default|Get3D%20Button%20Widget) (Utilities|Select :Index (Variables|Default|GetButton%20Type) :NewEnumerator0 "Play" :NewEnumerator1 "Settings" :NewEnumerator2 "Quit")))