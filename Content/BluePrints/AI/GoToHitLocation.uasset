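; GoToHitLocation is a behavior tree task that moves an AI-controlled pawn toward the LocationToMoveRobot position stored on the player character class MyCharacter.
; On execute, it reads that character from the blackboard, caches the position and sets ArriveDestination to true.
; Its AI tick issues SimpleMoveToLocation, then finishes immediately, setting ArriveDestination and success or failure by whether the pawn is within a fixed distance of the goal.
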(event EventReceiveTickAI
  (params (OwnerController :type AI%20Controller%20Object%20Reference) (ControlledPawn :type Pawn%20Object%20Reference) (DeltaSeconds :type Float%20%28single-precision%29))
  (bind _newpositiontomoverobot (Variables|Default|GetnewPositionToMoveRobot))
  (AI|Navigation|SimpleMovetoLocation OwnerController _newpositiontomoverobot)
  (if (> (Math|Vector|VectorLength (- (Transformation|GetActorLocation ControlledPawn) _newpositiontomoverobot)) 2.5e+02)
    (Class|BTFunctionLibrary|SetBlackboardValueasBool (Variables|Default|GetarriveDestination?) false)
    (AI|BehaviorTree|FinishExecute false)
    (else
      (Class|BTFunctionLibrary|SetBlackboardValueasBool (Variables|Default|GetarriveDestination?) true)
      (AI|BehaviorTree|FinishExecute true))))

(event EventReceiveExecute
  (params (OwnerActor :type Actor%20Object%20Reference))
  (bind _asmy_character (Utilities|Casting|CastToMyCharacter (AI|BehaviorTree|GetBlackboardValueasActor (Variables|Default|GetmyCharacterBlackboard))))
  (bind _output_get (Variables|Default|SetmyCharacterInAI _asmy_character))
  (Variables|Default|SetnewPositionToMoveRobot (Variables|/Game/BluePrints/Character/MyCharacter.MyCharacter_C|GetlocationToMoveRobot _output_get))
  (Class|BTFunctionLibrary|SetBlackboardValueasBool (Variables|Default|GetarriveDestination?) true))