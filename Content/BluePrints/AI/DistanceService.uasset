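; Behavior tree service that tracks whether the controlled pawn is farther than a set distance from a target actor.
; On each AI tick it measures the distance between the pawn and the actor stored in a blackboard key.
; It writes the result to the InRange blackboard bool, which is true when the distance exceeds MiniumDistance, and also prints it for debugging.
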(event EventReceiveTickAI
  (params (OwnerController :type AI%20Controller%20Object%20Reference) (ControlledPawn :type Pawn%20Object%20Reference) (DeltaSeconds :type Float%20%28single-precision%29))
  (bind _returnvalue (Transformation|GetActorLocation ControlledPawn))
  (bind _actorblackboard (Variables|Default|GetactorBlackboard))
  (bind _miniumdistance (Variables|Default|GetminiumDistance))
  (bind _returnvalue_2 (AI|BehaviorTree|GetBlackboardValueasActor _actorblackboard))
  (bind _returnvalue_3 (Transformation|GetActorLocation _returnvalue_2))
  (bind _returnvalue_4 (- _returnvalue _returnvalue_3))
  (bind _returnvalue_5 (Math|Vector|VectorLength _returnvalue_4))
  (bind _returnvalue_6 (> _returnvalue_5 _miniumdistance))
  (Class|BTFunctionLibrary|SetBlackboardValueasBool (Variables|Default|GetinRangeBlackboard) _returnvalue_6)
  (Development|PrintString (Utilities|String|ToString(Boolean) _returnvalue_6)))