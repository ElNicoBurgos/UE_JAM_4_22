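; Master sliding double-door actor with front and back terminals that show open or closed state.
; OpenDoorEvent sets IsOpen, swaps terminal materials and lights between green and red, plays a sound, and runs the OpenDoor timeline forward or reverse.
; The timeline lerps both panels apart along relative X.
; EnableOutlineEvent toggles a custom-depth stencil outline on the panels and prints a debug string.
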(event Custom|Enable%20Outline%20Event
  (params (Enable :type Boolean))
  (bind _door_left (Variables|Default|GetDoor-Left))
  (bind _door_right (Variables|Default|GetDoor_Right))
  (Development|PrintString (Utilities|String|ToString(Boolean) Enable) true true "(R=0.000000,G=0.660000,B=1.000000,A=1.000000)" 0.0)
  (if Enable
    (Rendering|SetCustomDepthStencilValue _door_left 1)
    (Rendering|SetRenderCustomDepth _door_left true)
    (else
      (Rendering|SetRenderCustomDepth _door_right false)
      (Rendering|SetCustomDepthStencilValue _door_right 0))))

(event Custom|Open%20Door%20Event
  (params (Open? :type Boolean))
  (Rendering|Components|Light|SetLightColor (Variables|Default|GetFront%20Terminal%20Light) (select Open? "(R=0.000000,G=1.000000,B=0.000000,A=1.000000)" "(R=1.000000,G=0.000000,B=0.000000,A=1.000000)") true)
  (Audio|PlaySound2D "/Game/SFX/Door_Open_1.Door_Open_1" 1.0 1.0 0.0 0 0)
  (if Open?
    (Rendering|Material|SetMaterial (Variables|Default|GetFront%20Terminal) 0 "/Game/Materials/Green_Emissive.Green_Emissive")
    (Variables|Default|SetIs%20Open true)
    (bind (_direction _lerp_alpha) (Timeline|Open%20Door Play)
      (:Update
        (Transformation|SetRelativeLocation (Variables|Default|GetDoor_Right) (Math|Vector|Lerp(Vector) "-36.666664,-28.333008,-36.666672" "68.333336,-28.332727,-36.666672" _lerp_alpha) false false)
        (Transformation|SetRelativeLocation (Variables|Default|GetDoor-Left) (Math|Vector|Lerp(Vector) "-36.666664,-28.333008,-36.666672" "-141.666656,-28.333569,-36.666672" _lerp_alpha) false false)))
    (else
      (Rendering|Material|SetMaterial (Variables|Default|GetBack%20Terminal) 0 "/Game/Materials/Red_Emission.Red_Emission")
      (Variables|Default|SetIs%20Open false)
      (Timeline|Open%20Door Reverse))))

(event EventBeginPlay
  (bind (_direction _lerp_alpha) (Timeline|Open%20Door SetNewTime)
    (:Update
      (Transformation|SetRelativeLocation (Variables|Default|GetDoor_Right) (Math|Vector|Lerp(Vector) "-36.666664,-28.333008,-36.666672" "68.333336,-28.332727,-36.666672" _lerp_alpha) false false)
      (Transformation|SetRelativeLocation (Variables|Default|GetDoor-Left) (Math|Vector|Lerp(Vector) "-36.666664,-28.333008,-36.666672" "-141.666656,-28.333569,-36.666672" _lerp_alpha) false false))))

(fn ConstructionScript)

(fn NewFunction0
  (return false))